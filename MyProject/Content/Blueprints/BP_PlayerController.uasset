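; Player controller Blueprint handling movement, a dash and a melee attack through Enhanced Input actions.
; Move input feeds world-axis movement on the pawn, while the jump action dashes it with a small upward launch then a forward launch, gated by a DoOnce cooldown.
; Attack runs a short forward sphere trace against pawns, drawing debug shapes and sending a damage message with a damage-info struct to the hit actor.
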(event Input|EnhancedActionEvents|EnhancedInputActionIA_Move
  (params (ActionValue :type Vector%202D%20Structure) (ElapsedSeconds :type Float%20%28double-precision%29) (TriggeredSeconds :type Float%20%28double-precision%29) (InputAction :type Input%20Action%20Object%20Reference :default "/Game/TopDownHybrid/Input/Actions/IA_Move.IA_Move"))
  (bind (_x _y) (Math|Vector2D|BreakVector2D ActionValue))
  ;[0.05098 0.05098 0.05098] Movement
  (Pawn|Input|AddMovementInput (Game|Player|GetPlayerPawn 0) "1.000000,0.000000,0.000000" _x false)
  (Pawn|Input|AddMovementInput (Game|Player|GetPlayerPawn 0) "0.000000,1.000000,0.000000" _y false))

(event Input|EnhancedActionEvents|EnhancedInputActionIA_Jump
  (params (ActionValue :type Boolean) (ElapsedSeconds :type Float%20%28double-precision%29) (TriggeredSeconds :type Float%20%28double-precision%29) (InputAction :type Input%20Action%20Object%20Reference :default "/Game/TopDownHybrid/Input/Actions/IA_Jump.IA_Jump"))
  ;[0.05098 0.05098 0.05098] Dash Input
  (:Started
    (Utilities|FlowControl|DoOnce false :!label _label
      (:Completed
        (Character|LaunchCharacter (Game|GetPlayerCharacter 0) "0.000000,0.000000,200.000000" false false)
        (Utilities|FlowControl|Delay 0.01)
        (Character|LaunchCharacter (Game|GetPlayerCharacter 0) (* (Math|Vector|GetForwardVector (Transformation|GetActorRotation (Game|Player|GetPlayerPawn 0))) 2e+03) false false)
        (Utilities|FlowControl|Delay 2.0)
        (goto _label Reset)))))

(event Input|EnhancedActionEvents|EnhancedInputActionIA_Attack
  (params (ActionValue :type Boolean) (ElapsedSeconds :type Float%20%28double-precision%29) (TriggeredSeconds :type Float%20%28double-precision%29) (InputAction :type Input%20Action%20Object%20Reference :default "/Game/TopDownHybrid/Input/Actions/IA_Attack.IA_Attack"))
  ;[0.15 0.15 0.15 0.5] Attack
  (:Started
    (CallFunction|Attack)))

(fn ConstructionScript)

(fn Attack
  (bind _returnvalue (Pawn|GetControlledPawn))
  (bind _returnvalue_2 (Transformation|GetActorLocation _returnvalue))
  (bind (_outhit _returnvalue_3) (Collision|SphereTraceForObjects _returnvalue_2 (+ (* (Transformation|GetActorForwardVector _returnvalue) 1e+02) _returnvalue_2) 2e+01 (Utilities|Array|MakeArray "ObjectTypeQuery3") false (Utilities|Array|MakeArray _returnvalue) "ForDuration" true "(R=1.000000,G=0.000000,B=0.000000,A=1.000000)" "(R=0.000000,G=1.000000,B=0.000000,A=1.000000)" 1.0))
  (if _returnvalue_3
    (Class|BPIDamagable|TakeDamage(Message) (.HitActor (Collision|BreakHitResult _outhit)) (Utilities|Struct|MakeS_DamageInfo 1e+01 "NewEnumerator1" "NewEnumerator1"))
    (Development|PrintString "Hit")))