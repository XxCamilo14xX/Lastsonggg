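; BP_Enemy is a damageable enemy character that forwards health, healing and damage calls to its BPCDamgeSystem component.
; Component events bound in the construction script trigger ragdoll on death and print block and damage feedback.
; An optional widget health bar has a looping timer, with logic to face the camera and set opacity by player distance.
; It also carries Enhanced Input movement, sprint and a hop-then-launch dash with cooldown, and replicates its sprite.
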(event Custom|DamagedType
  (params (DamagedType :type E_DamageType%20Enum :default "NewEnumerator0"))
  (Development|PrintString (Utilities|String|EnumtoString DamagedType)))

(event Custom|Death
  (bind _mesh (Variables|Character|GetMesh))
  (Physics|SetSimulatePhysics _mesh true)
  (Collision|SetCollisionEnabled _mesh "QueryAndPhysics"))

(event Custom|Blocked
  (params (CanBeParried :type Boolean))
  (Development|PrintString "Blocked"))

(event Custom|DamagedResponse
  (params (DamagedResponse :type E_DamageResponse%20Enum :default "NewEnumerator0"))
  (Development|PrintString (Utilities|String|EnumtoString DamagedResponse)))

(event Custom|BarControl
  (bind _healthbar (Variables|Default|GetHealthBar))
  (Transformation|SetWorldRotation _healthbar (Math|Rotator|FindLookatRotation (Transformation|GetWorldLocation _healthbar) (Camera|GetCameraLocation (Game|GetPlayerCameraManager 0))) false false)
  (Widget|SetRenderOpacity (UserInterface|GetUserWidgetObject (Variables|Default|GetHealthBar)) (Math|Float|MapRangeClamped (Math|Vector|Distance(Vector) (Transformation|GetActorLocation (Game|GetPlayerCharacter 0)) (Transformation|GetActorLocation)) 0.0 2e+03 1.0 0.0)))

(event Input|EnhancedActionEvents|EnhancedInputActionIA_Move
  (params (ActionValue :type Vector%202D%20Structure) (ElapsedSeconds :type Float%20%28double-precision%29) (TriggeredSeconds :type Float%20%28double-precision%29) (InputAction :type Input%20Action%20Object%20Reference :default "/Game/TopDownHybrid/Input/Actions/IA_Move.IA_Move"))
  (bind (_x _y) (Math|Vector2D|BreakVector2D ActionValue))
  ;[0.05098 0.05098 0.05098] Movement
  (Pawn|Input|AddMovementInput "1.000000,0.000000,0.000000" _x false)
  (Pawn|Input|AddMovementInput "0.000000,1.000000,0.000000" _y false))

(event Input|EnhancedActionEvents|EnhancedInputActionIA_Jump
  (params (ActionValue :type Boolean) (ElapsedSeconds :type Float%20%28double-precision%29) (TriggeredSeconds :type Float%20%28double-precision%29) (InputAction :type Input%20Action%20Object%20Reference :default "/Game/TopDownHybrid/Input/Actions/IA_Jump.IA_Jump"))
  ;[0.05098 0.05098 0.05098] Dash Input
  (:Started
    (Utilities|FlowControl|DoOnce false :!label _label
      (:Completed
        (Character|LaunchCharacter "0.000000,0.000000,200.000000" false false)
        (Utilities|FlowControl|Delay 0.01)
        (Character|LaunchCharacter (* (Math|Vector|GetForwardVector (Transformation|GetActorRotation)) 2e+03) false false)
        (Utilities|FlowControl|Delay 2.0)
        (goto _label Reset)))))

(event Input|EnhancedActionEvents|EnhancedInputActionIA_Sprint
  (params (ActionValue :type Boolean) (ElapsedSeconds :type Float%20%28double-precision%29) (TriggeredSeconds :type Float%20%28double-precision%29) (InputAction :type Input%20Action%20Object%20Reference :default "/Game/TopDownHybrid/Input/Actions/IA_Sprint.IA_Sprint"))
  ;[0 0 0 0] Sprint when holding button
  (:Started
    (Variables|Sprint|SetIsSprinting true)
    (Variables|/Script/Engine.CharacterMovementComponent|SetMaxWalkSpeed (Variables|Character|GetCharacterMovement) (Variables|Sprint|GetSprintSpeed)))
  (:Canceled
    (Variables|Sprint|SetIsSprinting false :!label _label)
    (Variables|/Script/Engine.CharacterMovementComponent|SetMaxWalkSpeed (Variables|Character|GetCharacterMovement) (Variables|Sprint|GetWalkSpeed)))
  (:Completed
    (goto _label)))

(event EventBeginPlay
  ;[0.05098 0.05098 0.05098] Init Enhanced Input and set Flipbook to replicated for multiplayer
  (CallFunction|InitInput)
  (Class|ActorComponent|SetIsReplicated (Variables|Default|GetSprite) true)
  ;[0.05098 0.05098 0.05098] Save walk speed from Character Movement Comp
  (Variables|Sprint|SetWalkSpeed (Variables|/Script/Engine.CharacterMovementComponent|GetMaxWalkSpeed (Variables|Character|GetCharacterMovement)))
  (if (Variables|Default|GethasHealthBar)
    (CallFunction|SetHealthBar)
    (Utilities|Time|SetTimerbyEvent (EventDispatchers|CreateEvent :!event Custom|BarControl) 0.0 true true)))

(event EventTick
  (params (DeltaSeconds :type Float%20%28single-precision%29)))

(fn ConstructionScript
  (bind _bpc_damgesystem (Variables|Default|GetBPC_DamgeSystem))
  (EventDispatchers|BindEventtoOnDeath _bpc_damgesystem (EventDispatchers|CreateEvent :!event Custom|Death))
  (EventDispatchers|BindEventtoOnBlocked _bpc_damgesystem (EventDispatchers|CreateEvent :!event Custom|Blocked))
  (EventDispatchers|BindEventtoOnDamagedResponse _bpc_damgesystem (EventDispatchers|CreateEvent :!event Custom|DamagedResponse))
  (EventDispatchers|BindEventtoOnDamagedType _bpc_damgesystem (EventDispatchers|CreateEvent :!event Custom|DamagedType)))

(fn InitInput
  (bind _asplayer_controller (Utilities|Casting|CastToPlayerController (Pawn|GetController))
    (:then
      (Input|AddMappingContext (PlayerController|LocalPlayerSubsystems|GetEnhancedInputLocalPlayerSubsystem _asplayer_controller) "/Game/TopDownHybrid/Input/IMC_Hybrid.IMC_Hybrid" 0 "(bIgnoreAllPressedKeysUntilRelease=True,bForceImmediately=False,bNotifyUserSettings=False)")
      (return))
    (:CastFailed
      (return))))

(fn SetHealthBar
  (bind _returnvalue (UserInterface|CreateWidget "/Game/Widgets/Wid/W_HealthBar.W_HealthBar_C" 0 self))
  (UserInterface|SetWidget (Variables|Default|GetHealthBar) _returnvalue))

(fn RefresHealthBar
  (bind _healthbar (Variables|Default|GetHealthBar))
  (bind _returnvalue (UserInterface|GetWidget _healthbar))
  (if (Variables|Default|GethasHealthBar)
    (Utilities|IsValid _returnvalue
      (:Is%20Valid
        (Class|BPIWidgetDatta|UpdateDatta(Message) _returnvalue)))))

(fn GetCurrentHealth
  (return (Variables|/Game/DamageSystem/BPC_DamgeSystem.BPC_DamgeSystem_C|GetHealth (Variables|Default|GetBPC_DamgeSystem))))

(fn GetMaxHealth
  (return (Variables|/Game/DamageSystem/BPC_DamgeSystem.BPC_DamgeSystem_C|GetMaxHealth (Variables|Default|GetBPC_DamgeSystem))))

(fn Heal
  (params (Amount :type Float%20%28double-precision%29))
  (bind _newhealth (Default|Heal (Variables|Default|GetBPC_DamgeSystem) Amount))
  (return _newhealth))

(fn TakeDamage
  (params (DamgeInfo :type S%20Damage%20Info%20Structure))
  (bind _wasdamaged (Default|TakeDamage (Variables|Default|GetBPC_DamgeSystem) DamgeInfo))
  (return _wasdamaged))